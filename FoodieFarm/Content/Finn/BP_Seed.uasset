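; BP_Seed is a seed actor that turns into a pumpkin when Finn's ZaniPlay flag is true while its box is overlapped.
; Unfiltered box overlap events set the Seedoverlap flag and toggle an arrow indicator, which Tick bobs with a sine offset while visible.
; Tick also polls both flags, then spawns an explosion effect and BP_Pumpkin, adds to Finn's EXP and destroys the seed.
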(event OnComponentBeginOverlap(Box)
  (params (OverlappedComponent :type Primitive%20Component%20Object%20Reference) (OtherActor :type Actor%20Object%20Reference) (OtherComp :type Primitive%20Component%20Object%20Reference) (OtherBodyIndex :type Integer) (bFromSweep :type Boolean) (SweepResult :type Hit%20Result%20Structure%20%28by%20ref%29))
  (Variables|Default|SetSeedoverlap true)
  (Rendering|SetVisibility (Variables|Default|GetArrow) true false))

(event OnComponentEndOverlap(Box)
  (params (OverlappedComponent :type Primitive%20Component%20Object%20Reference) (OtherActor :type Actor%20Object%20Reference) (OtherComp :type Primitive%20Component%20Object%20Reference) (OtherBodyIndex :type Integer))
  (Variables|Default|SetSeedoverlap false)
  (Rendering|SetVisibility (Variables|Default|GetArrow) false false))

(event EventBeginPlay
  (bind _asfinn (Utilities|Casting|CastToFinn (Game|Player|GetPlayerPawn 0)))
  (Variables|Default|SetAs%20Finn _asfinn))

(event Collision|EventActorBeginOverlap
  (params (OtherActor :type Actor%20Object%20Reference)))

(event EventTick
  (params (DeltaSeconds :type Float%20%28single-precision%29))
  (bind _returnvalue (Transformation|GetActorLocation))
  (bind _arrow (Variables|Default|GetArrow))
  (bind _as_finn (Variables|Default|GetAs%20Finn))
  (Utilities|FlowControl|Sequence
    (:then_0
      (if (and (Rendering|IsVisible _arrow) (Utilities|IsValid _arrow))
        (Transformation|AddLocalOffset (Variables|Default|GetArrow) (Math|Vector|MakeVector 0.0 0.0 (* (Math|Trig|Sin(Radians) (* (Utilities|Time|GetTimeSeconds) 7.0)) 0.4)) false false)))
    (:then_1
      (if (and (Variables|/Game/Finn/Finn.Finn_C|GetZaniPlay (Variables|Default|GetAs%20Finn)) (Variables|Default|GetSeedoverlap))
        (Effects|SpawnEmitteratLocation "/Game/StarterContent/Particles/P_Explosion.P_Explosion" (Transformation|GetActorLocation))
        (Game|SpawnActorfromClass "/Game/Finn/BP_Pumpkin.BP_Pumpkin_C" (Math|Transform|MakeTransform (Math|Vector|MakeVector (.x _returnvalue) (.y _returnvalue) (- (.z _returnvalue) 2e+01)) "0, 0, 0" "1.000000,1.000000,1.000000") "Undefined" "MultiplyWithRoot" 0 0)
        (Variables|/Game/Finn/Finn.Finn_C|SetEXP _as_finn (+ (Variables|/Game/Finn/Finn.Finn_C|GetEXP _as_finn) 0.1))
        (Actor|DestroyActor)))))

(fn ConstructionScript)