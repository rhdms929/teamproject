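; BP_Pumpkin is a breakable pumpkin that explodes and awards Finn experience when destroyed.
; It caches the player pawn as Finn, then checks every tick whether he is within close range with XaniPlay active.
; When both hold, it spawns an explosion, adds a small EXP amount and destroys itself.
; Box overlaps toggle PumpkinOverlap, but the distance check does not use that flag.
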(event OnComponentBeginOverlap(Box)
  (params (OverlappedComponent :type Primitive%20Component%20Object%20Reference) (OtherActor :type Actor%20Object%20Reference) (OtherComp :type Primitive%20Component%20Object%20Reference) (OtherBodyIndex :type Integer) (bFromSweep :type Boolean) (SweepResult :type Hit%20Result%20Structure%20%28by%20ref%29))
  (Variables|Default|SetPumpkinOverlap true))

(event OnComponentEndOverlap(Box)
  (params (OverlappedComponent :type Primitive%20Component%20Object%20Reference) (OtherActor :type Actor%20Object%20Reference) (OtherComp :type Primitive%20Component%20Object%20Reference) (OtherBodyIndex :type Integer))
  (Variables|Default|SetPumpkinOverlap false))

(event EventBeginPlay
  (bind _asfinn (Utilities|Casting|CastToFinn (Game|Player|GetPlayerPawn 0)))
  (Variables|Default|SetAs%20Finn _asfinn))

(event Collision|EventActorBeginOverlap
  (params (OtherActor :type Actor%20Object%20Reference)))

(event EventTick
  (params (DeltaSeconds :type Float%20%28single-precision%29))
  (bind _as_finn (Variables|Default|GetAs%20Finn))
  (if (and (< (Math|Vector|Distance(Vector) (Transformation|GetActorLocation (Variables|Default|GetAs%20Finn)) (Transformation|GetActorLocation)) 1.5e+02) (Variables|/Game/Finn/Finn.Finn_C|GetXaniPlay (Variables|Default|GetAs%20Finn)))
    (Effects|SpawnEmitteratLocation "/Game/StarterContent/Particles/P_Explosion.P_Explosion" (Transformation|GetActorLocation))
    (Variables|/Game/Finn/Finn.Finn_C|SetEXP _as_finn (+ (Variables|/Game/Finn/Finn.Finn_C|GetEXP _as_finn) 0.1))
    (Actor|DestroyActor)))

(fn ConstructionScript)